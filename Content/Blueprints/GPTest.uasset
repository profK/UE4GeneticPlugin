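; GPTest is a test Blueprint that exercises gene pool helper functions and prints the results.
; On BeginPlay it initializes a small GenePool, then reads back and prints its genome size and count through ExtractParameters.
; It then extracts each genome by index and concatenates its genes into a bracketed string, printing the length minus one, each intermediate string and the final result.
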(event EventBeginPlay
  (bind _genepool (Variables|Default|GetGenePool))
  (bind _returnvalue (Class|GenomePoolBPLibrary|InitializeGenePool (Variables|Default|GetGenePool) 5 5))
  (bind (_genomesize _genomecount) (Class|GenomePoolBPLibrary|ExtractParameters _returnvalue))
  (Development|PrintString (Utilities|String|ToString(Vector2d) (Math|Vector2D|MakeVector2D _genomesize _genomecount)))
  (bind _genomecount_2 (Class|GenomePoolBPLibrary|ExtractParameters _genepool))
  (for _index (range 0 (- (Math|Float|Truncate _genomecount_2) 1))
    (bind _returnvalue_2 (Class|GenomePoolBPLibrary|ExtractGenome _genepool _index))
    (Variables|Default|Setarraystring "[")
    (Development|PrintString (Utilities|String|ToString(Integer) (- (Utilities|Array|Length _returnvalue_2) 1)))
    (for _index_2 (range 0 (- (Utilities|Array|Length _returnvalue_2) 1))
      (bind _output_get (Variables|Default|Setarraystring (Utilities|String|Append (Variables|Default|Getarraystring) (Utilities|String|ToString(Float) (Utilities|Array|Get(acopy) _returnvalue_2 _index_2)) " ")))
      (Development|PrintString _output_get))
    (bind _output_get_2 (Variables|Default|Setarraystring (Utilities|String|Append _output_get "]")))
    (Development|PrintString _output_get_2)))